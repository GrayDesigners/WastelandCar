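; BP_PickupBase is a base weapon pickup that a character collects by walking into its sphere.
; On overlap, it fills the primary or secondary slot according to IsPrimaryWeapon if that slot is free, triggers a weapon swap and destroys itself.
; Equipped flags are set on player 0's character rather than the overlapping actor.
; Sphere collision stays disabled briefly after BeginPlay, delaying when pickup is possible.
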(event `self.Sphere.OnComponentBeginOverlap`
  (params (OverlappedComponent :type "PrimitiveComponent Object Reference") (OtherActor :type "Actor Object Reference") (OtherComp :type "PrimitiveComponent Object Reference") (OtherBodyIndex :type Integer) (bFromSweep :type Boolean) (SweepResult :type "HitResult Structure (by ref)"))
  (bind (_bsuccess _asfirst_person_character) (cast `` OtherActor :!pure true))
  (bind (_bsuccess_2 _asfirst_person_character_2) (cast `` (`GameplayStatics.GetPlayerCharacter` 0) :!pure true))
  ;[1 0.1843 0.1843] PickupBase
  (if _bsuccess
    (if true
      (if (`self.IsPrimaryWeapon`)
        (if (not (`/Game/TRASH/Bronie/BP_PickupBase.PrimaryWeaponEquip` _asfirst_person_character))
          (set `/Game/TRASH/Bronie/BP_PickupBase.PrimaryWeapon` (make `` (`self.WeaponName`) (`.WeaponClass` (`self.WeaponClass`))) _asfirst_person_character)
          (set `/Game/TRASH/Bronie/BP_PickupBase.WeaponEquipped` 0 _asfirst_person_character)
          (`self.WeaponSwap` _asfirst_person_character)
          (`self.K2_DestroyActor`)
          (set `/Game/TRASH/Bronie/BP_PickupBase.WeaponEquiped` true _asfirst_person_character_2)
          (set `/Game/TRASH/Bronie/BP_PickupBase.PrimaryWeaponEquip` true _asfirst_person_character_2))
        (elif (not (`/Game/TRASH/Bronie/BP_PickupBase.SecondaryWeaponEquip` _asfirst_person_character))
          (set `/Game/TRASH/Bronie/BP_PickupBase.SecondaryWeapon` (make `` (`self.WeaponName`)) _asfirst_person_character)
          (set `/Game/TRASH/Bronie/BP_PickupBase.WeaponEquipped` 1 _asfirst_person_character)
          (`self.WeaponSwap` _asfirst_person_character)
          (`self.K2_DestroyActor`)
          (set `/Game/TRASH/Bronie/BP_PickupBase.WeaponEquiped` true _asfirst_person_character_2)
          (set `/Game/TRASH/Bronie/BP_PickupBase.SecondaryWeaponEquip` true _asfirst_person_character_2))))))

(event `self.ReceiveBeginPlay`
  (bind _sphere (`self.Sphere`))
  ;[0.3922 0.4392 1] Collision
  (`PrimitiveComponent.SetCollisionEnabled` _sphere "NoCollision")
  (`KismetSystemLibrary.Delay` 0.5)
  (`PrimitiveComponent.SetCollisionEnabled` _sphere "QueryOnly"))

(fn `UserConstructionScript`)