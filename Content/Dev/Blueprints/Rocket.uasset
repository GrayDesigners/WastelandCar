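; Rocket is a projectile actor that explodes on contact and can home in on a target.
; On its first collision hit, it fires a radial force impulse, spawns an explosion particle effect at that force's location and destroys itself.
; The HomingMissile event takes a target and, if valid, points the projectile movement's homing at the target's static mesh with a fixed high acceleration.
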(event `self.CollisionComponent.OnComponentHit`
  (params (HitComponent :type "PrimitiveComponent Object Reference") (OtherActor :type "Actor Object Reference") (OtherComp :type "PrimitiveComponent Object Reference") (NormalImpulse :type "Vector Structure") (Hit :type "HitResult Structure (by ref)"))
  (bind _explosionforce (`self.ExplosionForce`))
  ;[1 1 1] Explode on contact
  (`/Engine/EditorBlueprintResources/StandardMacros.DoOnce` false
    (:`Completed`
      (`RadialForceComponent.FireImpulse` _explosionforce)
      (`GameplayStatics.SpawnEmitterAtLocation` "/Game/StarterContent/Particles/P_Explosion.P_Explosion" (`SceneComponent.K2_GetComponentLocation` _explosionforce))
      (`self.K2_DestroyActor`))))

(event `HomingMissile`
  (params (TargetToHit :type "StaticMeshActor Object Reference"))
  (bind _projectile (`self.Projectile`))
  ;[1 1 1] HomingMissile
  (if (`KismetSystemLibrary.IsValid` TargetToHit)
    (set `ProjectileMovementComponent.HomingTargetComponent` (`StaticMeshActor.StaticMeshComponent` TargetToHit) _projectile)
    (set `ProjectileMovementComponent.bIsHomingProjectile` true _projectile)
    (set `ProjectileMovementComponent.HomingAccelerationMagnitude` 25000.0 _projectile)))

(fn `UserConstructionScript`)