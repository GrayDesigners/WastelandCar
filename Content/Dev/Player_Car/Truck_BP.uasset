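; Player truck Blueprint that turns its WeaponBase to follow the camera's horizontal direction.
; Each Tick sets WeaponBase world rotation, taking yaw from a look-at rotation between the Camera and WeaponBase locations.
; Roll and pitch are copied from the Mesh, so the weapon base tilts with the truck body.
; The construction script is empty.
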(event `self.ReceiveTick`
  (params (DeltaSeconds :type "Float (single-precision)"))
  ;[1 1 1] obracanie kamery
  (`SceneComponent.K2_SetWorldRotation` (`self.WeaponBase`) (`KismetMathLibrary.MakeRotator` (.roll (`SceneComponent.K2_GetComponentRotation` (`self.Mesh`))) (.pitch (`SceneComponent.K2_GetComponentRotation` (`self.Mesh`))) (.yaw (`KismetMathLibrary.FindLookAtRotation` (`SceneComponent.K2_GetComponentLocation` (`self.Camera`)) (`SceneComponent.K2_GetComponentLocation` (`self.WeaponBase`))))) false false))

(fn `UserConstructionScript`)